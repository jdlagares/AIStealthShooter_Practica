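; Player character Blueprint that handles crosshair display and feedback for health changes.
; BeginPlay adds a crosshair widget to the viewport, while Tick prints current health every frame as debug output.
; The HealthComponent's OnHealthChanged event answers damage with a world camera shake at the camera and a newly created hurt-screen widget.
; Any non-negative change only prints a "Healed:" message.
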(event OnHealthChanged(HealthComponent)
  (params (HealthComp :type AIP%20Health%20Component%20Object%20Reference) (Health :type Float%20%28single-precision%29) (HealthDelta :type Float%20%28single-precision%29) (DamageType :type Damage%20Type%20Object%20Reference) (InstigatedBy :type Controller%20Object%20Reference) (DamageCauser :type Actor%20Object%20Reference))
  (if (< HealthDelta 0.0)
    (Camera|PlayWorldCameraShake "/Game/FX/HitCameraShake.HitCameraShake_C" (Transformation|GetWorldLocation (Variables|Default|GetCamera)) 0.0 5e+01)
    (bind _returnvalue (UserInterface|CreateWidget "/Game/FX/WID_HurtScreen.WID_HurtScreen_C"))
    (UserInterface|Viewport|AddtoViewport _returnvalue 0)
    (else
      (Development|PrintString (Utilities|String|Append "Healed:" (Utilities|String|ToString(Float) HealthDelta))))))

(event EventBeginPlay
  (bind _returnvalue (UserInterface|CreateWidget "/Game/FX/CrossHair.CrossHair_C"))
  (UserInterface|Viewport|AddtoViewport _returnvalue 0))

(event Collision|EventActorBeginOverlap
  (params (OtherActor :type Actor%20Object%20Reference)))

(event EventTick
  (params (DeltaSeconds :type Float%20%28single-precision%29))
  (Development|PrintString (Utilities|String|ToString(Float) (Variables|/Script/ARK_StealthShooter.AIP_HealthComponent|GetCurrentHealth (Variables|Default|GetHealthComponent)))))

(fn ConstructionScript)