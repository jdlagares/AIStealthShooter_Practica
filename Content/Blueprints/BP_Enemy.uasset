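; Enemy Blueprint that displays health and AI alert state through in-world text.
; HealthComponent events update the color-banded health readout and, on death, hide it and stop the AI controller's brain logic.
; Point damage is forwarded as an AI damage sense event so perception can register the causer.
; SetEnemyStatus maps Patrol, Seek and Combat to a colored symbol, while Tick draws a debug forward arrow.
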(event OnHealthChanged(HealthComponent)
  (params (HealthComp :type AIP%20Health%20Component%20Object%20Reference) (Health :type Float%20%28single-precision%29) (HealthDelta :type Float%20%28single-precision%29) (DamageType :type Damage%20Type%20Object%20Reference) (InstigatedBy :type Controller%20Object%20Reference) (DamageCauser :type Actor%20Object%20Reference))
  (Rendering|Components|TextRender|SetText (Variables|Default|GetHealthText) (Utilities|Text|ToText(Float) Health "HalfToEven"))
  (Rendering|Components|TextRender|SetTextRenderColor (Variables|Default|GetHealthText) (CallFunction|GetColorfromHealth Health)))

(event OnDeath(HealthComponent)
  (params (HealthComp :type AIP%20Health%20Component%20Object%20Reference) (InstigatedBy :type Controller%20Object%20Reference) (Killer :type Actor%20Object%20Reference))
  (Rendering|SetVisibility (Variables|Default|GetHealthText) false false)
  (AI|Logic|StopLogic (Variables|/Script/AIModule.AIController|GetBrainComponent (AI|GetAIController self)) "Died"))

(event Custom|ReportPointDamage
  (params (DamagedActor :type Actor%20Object%20Reference) (Damage :type Float%20%28single-precision%29) (InstigatedBy :type Controller%20Object%20Reference) (HitLocation :type Vector) (FHitComponent :type Primitive%20Component%20Object%20Reference) (BoneName :type Name) (ShotFromDirection :type Vector) (DamageType :type Damage%20Type%20Object%20Reference) (DamageCauser :type Actor%20Object%20Reference))
  (Class|AISenseDamage|ReportDamageEvent DamagedActor DamageCauser Damage HitLocation "0, 0, 0" "None"))

(event EventBeginPlay
  (Rendering|Components|TextRender|SetText (Variables|Default|GetHealthText) (Utilities|Text|ToText(Float) (Variables|/Script/ARK_StealthShooter.AIP_HealthComponent|GetCurrentHealth (Variables|Default|GetHealthComponent)) "HalfToEven"))
  (Rendering|Components|TextRender|SetTextRenderColor (Variables|Default|GetHealthText) (Variables|Default|GetHealthyColor))
  (EventDispatchers|BindEventtoOnTakePointDamage (EventDispatchers|CreateEvent :!event Custom|ReportPointDamage)))

(event Collision|EventActorBeginOverlap
  (params (OtherActor :type Actor%20Object%20Reference)))

(event EventSetEnemyStatus
  (params (NewEnemyStatus :type EAIP_EnemyStatus%20Enum :default "EnemyStatus_Patrol"))
  (Rendering|Components|TextRender|SetText (Variables|Default|GetStatusText) (Utilities|Text|ToText(Name) (Utilities|Select :Index NewEnemyStatus :EnemyStatus_Patrol (Utilities|Name|MakeLiteralName "") :EnemyStatus_Finding (Utilities|Name|MakeLiteralName "?") :EnemyStatus_Combat (Utilities|Name|MakeLiteralName "!"))))
  (Rendering|Components|TextRender|SetTextRenderColor (Variables|Default|GetStatusText) (Utilities|Select :Index NewEnemyStatus :EnemyStatus_Patrol (Variables|Default|GetPatrolColor) :EnemyStatus_Finding (Variables|Default|GetSeekColor) :EnemyStatus_Combat (Variables|Default|GetCombatColor))))

(event EventTick
  (params (DeltaSeconds :type Float%20%28single-precision%29))
  (Rendering|Debug|DrawDebugArrow :LineEnd (* (Transformation|GetActorForwardVector) 1e+03) :ArrowSize 5e+01 :Duration 0.1 :Thickness 1e+01))

(fn ConstructionScript)

(fn GetColorfromHealth
  (params (Health :type Float%20%28single-precision%29))
  (if (> Health 8e+01)
    (return (Variables|Default|GetHealthyColor))
    (elif (> Health 5e+01)
      (return (Variables|Default|GetHurtColor))
      (else
        (return (Variables|Default|GetCriticalColor))))))